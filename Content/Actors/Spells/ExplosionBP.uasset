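; Explosion spell actor that follows the player and detonates after a charge-up of about five seconds, damaging nearby enemies.
; Tick keeps its Sphere on the player's location while BeginPlay plays the charge sound, waits, then shows the particle system and spawns the blast effect and sound.
; Damage comes from distance checks over all EnemyBasic and EnemyZombie actors rather than overlaps; zombies receive a zero source point.
; The actor destroys itself shortly afterwards.
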(event EventBeginPlay
  (bind _returnvalue (Game|Player|GetPlayerPawn 0))
  (bind _sphere (Variables|Default|GetSphere))
  (bind _returnvalue_2 (Transformation|GetWorldLocation _sphere))
  (bind _returnvalue_3 (Transformation|GetActorLocation _returnvalue))
  ;[1 1 1] Exploze po nabití
  (Audio|PlaySoundatLocation "/Game/Audio/tornado.tornado" _returnvalue_3 "0, 0, 0" 1.0 1.0 27.0 0 0 0)
  (Utilities|FlowControl|Delay 4.9)
  (Development|SetHiddeninGame (Variables|Default|GetParticleSystem) false false)
  (Audio|PlaySoundatLocation "/Game/Audio/mixkit-fire-spell-with-explosion-1338.mixkit-fire-spell-with-explosion-1338" _returnvalue_3 "0, 0, 0" 1.0 1.0 0.0 0 0 0)
  (Effects|SpawnEmitteratLocation "/Game/ContentPacks/FXVarietyPack/Particles/spell_explosion.spell_explosion" _returnvalue_3 "0, 0, 0" "0.800000,0.800000,0.700000")
  (bind _outactors (Actor|GetAllActorsOfClass "/Game/Characters/EnemyBasic.EnemyBasic_C"))
  (for _array_element _outactors
    (if (<= (Math|Vector|Distance(Vector) (Transformation|GetWorldLocation (Variables|/Script/Engine.Actor|GetRootComponent _array_element)) _returnvalue_2) 3e+02)
      (Default|TakeDamage _array_element 3e+01 _returnvalue_2)))
  (bind _outactors_2 (Actor|GetAllActorsOfClass "/Game/Characters/EnemyZombie.EnemyZombie_C"))
  (for _array_element_2 _outactors_2
    (if (<= (Math|Vector|Distance(Vector) (Transformation|GetWorldLocation (Variables|/Script/Engine.Actor|GetRootComponent _array_element_2)) (Transformation|GetWorldLocation (Variables|Default|GetSphere))) 3e+02)
      (Default|TakeDamage _array_element_2 3e+01 "0, 0, 0")))
  (Utilities|FlowControl|Delay 0.5)
  (Actor|DestroyActor))

(event Collision|EventActorBeginOverlap
  (params (OtherActor :type Actor%20Object%20Reference)))

(event EventTick
  (params (DeltaSeconds :type Float%20%28single-precision%29))
  ;[1 1 1] Posun zároveň s hráčem
  (Transformation|SetWorldLocation (Variables|Default|GetSphere) (Transformation|GetActorLocation (Game|Player|GetPlayerPawn 0)) false false))

(fn ConstructionScript)