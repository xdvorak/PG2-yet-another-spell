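; Player fireball spell projectile that flies straight along the player pawn's forward direction, captured at spawn.
; BeginPlay plays one of three random cast sounds and stores the direction.
; Tick moves the actor with a swept world offset scaled by Speed and delta time.
; A blocking hit or actor overlap spawns a shockwave emitter, plays a surroundings or enemy impact sound respectively, and destroys the fireball.
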(event EventBeginPlay
  ;[1 1 1] určení směru letu po vytvoření
  (switch int (Math|Random|RandomIntegerinRange 0 2)
    (:0
      (Audio|SpawnSound2D "/Game/Audio/Fireball_Bluezone_BC0261_mountain_dweller_texture_fire_whoosh_003.Fireball_Bluezone_BC0261_mountain_dweller_texture_fire_whoosh_003" 0.2 1.0 0.5 0))
    (:1
      (Audio|SpawnSound2D "/Game/Audio/fire-burst.fire-burst" 0.5 1.0 0.0 0))
    (:2
      (Audio|SpawnSound2D "/Game/Audio/fireball-cast-1.fireball-cast-1" 1.0 1.0 1.0 0)))
  (Variables|Default|Setdirection (Transformation|GetActorForwardVector (Game|Player|GetPlayerPawn 0))))

(event Collision|EventActorBeginOverlap
  (params (OtherActor :type Actor%20Object%20Reference))
  (bind _sphere (Variables|Default|GetSphere))
  (bind _returnvalue (Transformation|GetWorldLocation _sphere))
  ;[1 1 1] zásah postavy
  (Effects|SpawnEmitteratLocation "/Game/ContentPacks/FXVarietyPack/Particles/P_ky_shotShockwave.P_ky_shotShockwave" _returnvalue "0, 0, 0" "0.300000,0.300000,0.300000")
  (Audio|PlaySoundatLocation "/Game/Audio/fireball-enemy-hit.fireball-enemy-hit" _returnvalue "0, 0, 0" 1.0 1.0 0.0 0 0 0)
  (Actor|DestroyActor))

(event EventTick
  (params (DeltaSeconds :type Float%20%28single-precision%29))
  ;[1 1 1] posun ve směru letu
  (Transformation|AddActorWorldOffset (* (Variables|Default|Getdirection) (* (Variables|Default|GetSpeed) DeltaSeconds)) true))

(event Collision|EventHit
  (params (MyComp :type Primitive%20Component%20Object%20Reference) (Other :type Actor%20Object%20Reference) (OtherComp :type Primitive%20Component%20Object%20Reference) (bSelfMoved :type Boolean) (HitLocation :type Vector :default "0, 0, 0") (HitNormal :type Vector :default "0, 0, 0") (NormalImpulse :type Vector :default "0, 0, 0") (Hit :type Hit%20Result%20Structure%20%28by%20ref%29))
  ;[1 1 1] zásah čehokoliv
  (Effects|SpawnEmitteratLocation "/Game/ContentPacks/FXVarietyPack/Particles/P_ky_shotShockwave.P_ky_shotShockwave" HitLocation "0, 0, 0" "0.300000,0.300000,0.300000")
  (Audio|PlaySoundatLocation "/Game/Audio/fireball-surrounding-hit.fireball-surrounding-hit" HitLocation "0, 0, 0" 1.5 1.0 0.0 0 0 0)
  (Actor|DestroyActor))

(fn ConstructionScript)